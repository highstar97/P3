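; Anim notify state that detects and applies melee weapon hits during an attack animation window.
; Each tick sphere-traces between the owner weapon's base and tip sockets, using the weapon's radius, and collects hit P3Characters in a set cleared at begin.
; Notify end applies damage once to each collected character, with the owner as instigator.
; Debug trace drawing and damage prints are left on.
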(fn `Received_NotifyBegin`
  (params (MeshComp :type "SkeletalMeshComponent Object Reference") (Animation :type "AnimSequenceBase Object Reference") (TotalDuration :type "Float (single-precision)") (EventReference :type "AnimNotifyEventReference Structure (by ref)"))
  (returns (ReturnValue :type Boolean))
  (`BlueprintSetLibrary.Set_Clear` (`self.P3Characters`))
  (return false))

(fn `Received_NotifyEnd`
  (params (MeshComp :type "SkeletalMeshComponent Object Reference") (Animation :type "AnimSequenceBase Object Reference") (EventReference :type "AnimNotifyEventReference Structure (by ref)"))
  (returns (ReturnValue :type Boolean))
  (bind _result (`BlueprintSetLibrary.Set_ToArray` (`self.P3Characters`)))
  (for _array_element _result
    (bind _asp3character (cast `P3Character` (`ActorComponent.GetOwner` MeshComp))
      (:`then`
        (bind _returnvalue (`P3Character.ApplyDamage` _array_element (`Pawn.GetController` _asp3character) _asp3character))
        (`KismetSystemLibrary.PrintString` null (`KismetStringLibrary.Conv_DoubleToString` _returnvalue)))
      (:`CastFailed`
        (`KismetSystemLibrary.PrintString` null "[AnimNotify_MeleeAttack] Animation owner can't cast to P3Character."))))
  (return false))

(fn `Received_NotifyTick`
  (params (MeshComp :type "SkeletalMeshComponent Object Reference") (Animation :type "AnimSequenceBase Object Reference") (FrameDeltaTime :type "Float (single-precision)") (EventReference :type "AnimNotifyEventReference Structure (by ref)"))
  (returns (ReturnValue :type Boolean))
  (bind _weapon (`P3WeaponComponent.Weapon` (`P3Character.WeaponComponent` (cast `P3Character` (`ActorComponent.GetOwner` MeshComp) :!pure true))))
  (bind _rootcomponent (`Actor.RootComponent` _weapon))
  (bind (_outhits _returnvalue) (`KismetSystemLibrary.SphereTraceMultiForObjects` :`WorldContextObject` MeshComp :`Start` (`SceneComponent.GetSocketLocation` _rootcomponent "FX_weapon_base") :`End` (`SceneComponent.GetSocketLocation` _rootcomponent "FX_weapon_tip") :`Radius` (`P3Weapon.Radius` _weapon) :`ObjectTypes` (`|MakeArray` "ObjectTypeQuery7" "ObjectTypeQuery8" "ObjectTypeQuery3" :!type "EObjectTypeQuery Enum") :`DrawDebugType` "ForDuration" :`DrawTime` 2.0))
  (if _returnvalue
    (for _array_element _outhits
      (bind _asp3character (cast `P3Character` (`.HitActor` (`GameplayStatics.BreakHitResult` _array_element)))
        (:`then`
          (`BlueprintSetLibrary.Set_Add` (`self.P3Characters`) _asp3character))
        (:`CastFailed`
          (`KismetSystemLibrary.PrintString` null "[AnimNotify_MeleeAttack] Hit Actor can't cast to P3Character."))))
    (return false)))